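; RounderCmp_BP is a denoiser Blueprint, named as a component, that rounds float and transform values to the precision set by DecimalPosition.
; RoundFloat scales a value by a power of ten, rounds it to an integer, then divides back.
; RoundTransform applies RoundFloat to each location and rotation axis, leaving scale untouched.
; Its event graph is inactive, so it only offers these functions for other code to call.
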(fn `RoundFloat`
  (params (Float :type "Float (double-precision)"))
  (returns (RoundedFloat :type "Float (double-precision)"))
  (bind _returnvalue (`KismetMathLibrary.MultiplyMultiply_FloatFloat` 10.0 (`KismetMathLibrary.Conv_IntToDouble` (`self.DecimalPosition`))))
  (return (/ (`KismetMathLibrary.Conv_IntToDouble` (`KismetMathLibrary.Round` (* Float _returnvalue))) _returnvalue)))

(fn `RoundTransform`
  (params (Transform :type "Transform Structure"))
  (returns (RoundedTransform :type "Transform Structure"))
  (return (`KismetMathLibrary.MakeTransform` (`KismetMathLibrary.MakeVector` (`self.RoundFloat` (.x (.location Transform))) (`self.RoundFloat` (.y (.location Transform))) (`self.RoundFloat` (.z (.location Transform)))) (`KismetMathLibrary.MakeRotator` (`self.RoundFloat` (.roll (.rotation Transform))) (`self.RoundFloat` (.pitch (.rotation Transform))) (`self.RoundFloat` (.yaw (.rotation Transform)))) (.scale Transform))))