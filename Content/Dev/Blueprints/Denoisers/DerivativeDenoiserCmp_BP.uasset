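; Denoiser component that provides a stabilized transform of its owning actor by holding a cached location and rotation between updates.
; It caches the transform on BeginPlay, then refreshes it on Tick once the time threshold has elapsed.
; A location-threshold check runs only after that refresh, so updates are effectively time-gated rather than movement-filtered.
; GetStabilizedTransform returns the cached location and rotation with the owner's live scale.
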(event `self.ReceiveBeginPlay`
  (`self.UpdateTransform`))

(event `self.ReceiveTick`
  (params (DeltaSeconds :type "Float (single-precision)"))
  ;[1 1 1] If more time than the threshold has passed, update
  (if (>= (- (`GameplayStatics.GetTimeSeconds`) (`self.LastUpdateTime`)) (`self.TimeThreshold`))
    (`self.UpdateTransform`)
    ;[1 1 1] If the distance between the current location and LastLocation is lower than the threshold, update
    (if (<= (`KismetMathLibrary.VSize` (- (`self.LastLocation`) (`Actor.K2_GetActorLocation` (`self.GetOwner`)))) (`self.LocationThreshold`))
      (`self.UpdateTransform`))))

(fn `GetStabilizedTransform`
  (returns (Trasnform :type "Transform Structure"))
  (return (`KismetMathLibrary.MakeTransform` (`self.LastLocation`) (`self.LastRotation`) (`Actor.GetActorScale3D` (`self.GetOwner`)))))

(fn `UpdateTransform`
  (bind _returnvalue (`self.GetOwner`))
  (set `self.LastLocation` (`Actor.K2_GetActorLocation` _returnvalue))
  (set `self.LastRotation` (`Actor.K2_GetActorRotation` _returnvalue))
  (set `self.LastUpdateTime` (`GameplayStatics.GetTimeSeconds`)))